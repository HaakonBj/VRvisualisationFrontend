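; RestActor Blueprint that loads a history from MongoDB and spawns a CommitActor_BP for each entry.
; Its construction script calls InitRestActor and RestActorReady, which polls the Database with Delay loops until it is ready and, after requesting retrieval, has data.
; DataRetrieved spawns each actor at a diagonally stepped position, initializes it with its entry, stores it in CommitArray and prints the entry's strings.
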(event `RestActorReady`
  (bind _database (`self.database`))
  (if (`SqlConnect.DatabaseIsReady` _database) :!label _label
    (`self.RetrieveDataFromMongoDB`)
    (if (`SqlConnect.DatabaseGotData` _database) :!label _label_2
      (`self.DataRetrieved`)
      (else
        (`KismetSystemLibrary.Delay` 2.0)
        (goto _label_2)))
    (else
      (`KismetSystemLibrary.Delay` 2.0)
      (goto _label))))

(event `DataRetrieved`
  (bind _tempcommit (`self.TempCommit`))
  (bind _returnvalue (`SqlConnect.RetrieveWholeHistory` (`self.database`)))
  (for _array_element _returnvalue
    (`|ExecutionSequence`
      (:`then_0`
        (bind _output_get (set `self.Position` (`KismetMathLibrary.MakeVector` (+ (.x (`self.Position`)) -5.0) (+ (.y (`self.Position`)) -5.0) (+ (.z (`self.Position`)) -5.0)))))
      (:`then_1`
        (set `self.NewTransform` (`KismetMathLibrary.MakeTransform` _output_get)))
      (:`then_2`
        (bind _returnvalue_2 (`|SpawnActorFromClass` "/Game/Blueprints/CommitActor_BP.CommitActor_BP_C" (`self.NewTransform`) "AlwaysSpawn" "OverrideRootScale"))
        (set `self.TempCommit` _returnvalue_2))
      (:`then_3`
        (`CommitActor.Init` _tempcommit _array_element))
      (:`then_4`
        (`KismetArrayLibrary.Array_Add` (`self.CommitArray`) _tempcommit))
      (:`then_5`
        (for _array_element_2 (`.arr` (break `Arr` _array_element))
          (`KismetSystemLibrary.PrintString` _array_element_2)))))
  (`KismetSystemLibrary.PrintString` "I am done"))

(fn `UserConstructionScript`
  (`self.InitRestActor`)
  (`self.RestActorReady`))