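; HandCommitMenu is a menu, by name hand-mounted, that shows details of a version-control commit through four 3D icons.
; BeginPlay spawns hidden key, head, calendar and arrow actors, attaches them to the root and binds their display events.
; SetCommitObject stores the commit and reveals the icons.
; Each icon's event writes the hash, author, date or two parents into one shared TextRender, with date also printed for debugging.
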(event `SetText`
  (`TextRenderComponent.K2_SetText` (`self.TextRender`) (`KismetTextLibrary.Conv_StringToText` (`CommitActor.GetSha` (`self.Commit`)))))

(event `self.ReceiveBeginPlay`
  (bind _returnvalue (`KismetMathLibrary.MakeTransform` (0.0 0.0 0.0) (struct)))
  (bind _keymesh (`/Game/Blueprints/KeyActor.KeyMesh` (`self.KeyActor`)))
  (bind _arrow (`/Game/Blueprints/ArrowActor.Arrow` (`self.ArrowActor`)))
  (bind _child (`/Game/Blueprints/ArrowActor.child` (`self.ArrowActor`)))
  (bind _head (`/Game/Blueprints/HeadActor.Head` (`self.HeadActor`)))
  (bind _calendar (`/Game/Blueprints/CalendarActor.Calendar` (`self.CalendarActor`)))
  (`|ExecutionSequence`
    (:`then_0`
      (`|ExecutionSequence`
        (:`then_0`
          (bind _returnvalue_2 (`|SpawnActorFromClass` "/Game/Blueprints/KeyActor.KeyActor_C" _returnvalue "AlwaysSpawn" "OverrideRootScale"))
          (bind _output_get (set `self.KeyActor` _returnvalue_2))
          (`self.K2_AttachToComponent` _output_get (`self.DefaultSceneRoot`) "None" "SnapToTarget" "SnapToTarget" "KeepRelative" true)
          (`SceneComponent.K2_SetRelativeLocationAndRotation` _keymesh (0.0 0.0 -20.0) (struct :`Pitch` -30.0) false false)
          (`SceneComponent.SetVisibility` _keymesh false false))
        (:`then_1`
          (bind _returnvalue_3 (`|SpawnActorFromClass` "/Game/Blueprints/HeadActor.HeadActor_C" _returnvalue "AlwaysSpawn" "OverrideRootScale"))
          (bind _output_get_2 (set `self.HeadActor` _returnvalue_3))
          (`self.K2_AttachToComponent` _output_get_2 (`self.DefaultSceneRoot`) "None" "SnapToTarget" "SnapToTarget" "KeepRelative" true)
          (`SceneComponent.K2_SetRelativeLocation` _head (0.0 20.0 -20.0) false false)
          (`SceneComponent.K2_SetRelativeRotation` _head (struct :`Pitch` -180.0 :`Yaw` 90.0 :`Roll` -30.0) false false)
          (`SceneComponent.SetVisibility` _head false false))
        (:`then_2`
          (bind _returnvalue_4 (`|SpawnActorFromClass` "/Game/Blueprints/CalendarActor.CalendarActor_C" _returnvalue "AlwaysSpawn" "OverrideRootScale"))
          (bind _output_get_3 (set `self.CalendarActor` _returnvalue_4))
          (`self.K2_AttachToComponent` _output_get_3 (`self.DefaultSceneRoot`) "None" "KeepRelative" "KeepRelative" "KeepRelative" true)
          (`SceneComponent.K2_SetRelativeLocationAndRotation` _calendar (0.0 40.0 -20.0) (struct :`Pitch` -180.0 :`Yaw` 90.0 :`Roll` 30.0) false false)
          (`SceneComponent.SetVisibility` _calendar false false))
        (:`then_3`
          (bind _returnvalue_5 (`|SpawnActorFromClass` "/Game/Blueprints/ArrowActor.ArrowActor_C" _returnvalue "AlwaysSpawn" "OverrideRootScale"))
          (bind _output_get_4 (set `self.ArrowActor` _returnvalue_5))
          (`self.K2_AttachToComponent` _output_get_4 (`self.DefaultSceneRoot`) "None" "SnapToTarget" "SnapToTarget" "KeepRelative" true)
          (`SceneComponent.K2_SetRelativeLocationAndRotation` _arrow (0.0 -20.0 -20.0) (struct :`Pitch` -180.0 :`Yaw` 90.0 :`Roll` -30.0) false false)
          (`SceneComponent.SetVisibility` _arrow false false)
          (`SceneComponent.K2_SetRelativeLocationAndRotation` _child (0.0 -24.810471 -19.0) (struct :`Pitch` -180.0 :`Yaw` 90.0 :`Roll` -30.0) false false)
          (`SceneComponent.SetVisibility` _child false false))))
    (:`then_1`
      (add `/Game/Blueprints/KeyActor.DisplayCommitHash` (`self.KeyActor`) (delegate `SetText`)))
    (:`then_2`
      (add `/Game/Blueprints/HeadActor.DisplayAuthor` (`self.HeadActor`) (delegate `SetAuthor`)))
    (:`then_3`
      (add `/Game/Blueprints/CalendarActor.DisplayDate` (`self.CalendarActor`) (delegate `SetDate`)))
    (:`then_4`
      (add `/Game/Blueprints/ArrowActor.DisplayParents` (`self.ArrowActor`) (delegate `SetParents`)))))

(event `SetAuthor`
  (`TextRenderComponent.K2_SetText` (`self.TextRender`) (`KismetTextLibrary.Conv_StringToText` (`CommitActor.GetAuthor` (`self.Commit`)))))

(event `SetDate`
  (bind _returnvalue (`CommitActor.GetDate` (`self.Commit`)))
  (`KismetSystemLibrary.PrintString` _returnvalue)
  (`TextRenderComponent.K2_SetText` (`self.TextRender`) (`KismetTextLibrary.Conv_StringToText` _returnvalue)))

(event `SetParents`
  (bind _commit (`self.Commit`))
  (bind _output_get (set `self.Parents` (`KismetStringLibrary.Concat_StrStr` (`CommitActor.GetParentOne` _commit) "<br>" (`CommitActor.GetParentTwo` _commit))))
  (`TextRenderComponent.K2_SetText` (`self.TextRender`) (`KismetTextLibrary.Conv_StringToText` _output_get)))

(fn `SetCommitObject`
  (params (Commit :type "CommitActor Object Reference"))
  (set `self.Commit` Commit)
  (`|ExecutionSequence`
    (:`then_0`
      (`SceneComponent.SetVisibility` (`/Game/Blueprints/KeyActor.KeyMesh` (`self.KeyActor`)) true false))
    (:`then_1`
      (`SceneComponent.SetVisibility` (`/Game/Blueprints/HeadActor.Head` (`self.HeadActor`)) true false))
    (:`then_2`
      (`SceneComponent.SetVisibility` (`/Game/Blueprints/CalendarActor.Calendar` (`self.CalendarActor`)) true false))
    (:`then_3`
      (`SceneComponent.SetVisibility` (`/Game/Blueprints/ArrowActor.Arrow` (`self.ArrowActor`)) true false)
      (`SceneComponent.SetVisibility` (`/Game/Blueprints/ArrowActor.child` (`self.ArrowActor`)) true false))))

(fn `UserConstructionScript`)