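; VR-style lever actor that, while held, raises or lowers a referenced Floor actor and NavMesh actor.
; Pickup stores the grabbing hand component and Drop releases it.
; While grabbed, Tick points the lever at the hand in the XZ plane with a pitch offset.
; The sign of the lever's yaw then sets a fixed per-frame, frame-rate-dependent Z step for both actors, and the NavMesh height prints for debugging.
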(event `/Game/VirtualRealityBP/Blueprints/PickupActorInterface.Pickup`
  (params (AttachTo :type "SceneComponent Object Reference"))
  (set `self.Grabbed` true)
  (bind _output_get (set `self.ControllerHand` AttachTo))
  (set `self.OldPosition` (`SceneComponent.K2_GetComponentLocation` _output_get)))

(event `/Game/VirtualRealityBP/Blueprints/PickupActorInterface.Drop`
  (set `self.Grabbed` false))

(event `self.ReceiveTick`
  (params (DeltaSeconds :type "Float (single-precision)"))
  (bind (_returnvalue_roll _returnvalue_pitch _returnvalue_yaw) (`KismetMathLibrary.BreakRotator` (`self.K2_GetActorRotation`)))
  (bind _floor (`self.Floor`))
  (bind _navmesh (`self.NavMesh`))
  (bind (_returnvalue_x _returnvalue_y _returnvalue_z) (`KismetMathLibrary.BreakVector` (`self.K2_GetActorLocation` _navmesh)))
  (bind (_returnvalue_x_2 _returnvalue_y_2 _returnvalue_z_2) (`KismetMathLibrary.BreakVector` (`self.K2_GetActorLocation` _floor)))
  (bind (_returnvalue_x_3 _returnvalue_y_3 _returnvalue_z_3) (`KismetMathLibrary.BreakVector` (`self.K2_GetActorLocation` (`self.NavMesh`))))
  (if (`self.Grabbed`)
    (`|ExecutionSequence`
      (:`then_0`
        (`self.K2_SetActorRotation` (`KismetMathLibrary.MakeRotator` (.roll (`KismetMathLibrary.Conv_VectorToRotator` (`KismetMathLibrary.GreaterGreater_VectorRotator` (`KismetMathLibrary.Normal` (* (- (`SceneComponent.K2_GetComponentLocation` (`self.ControllerHand`)) (`self.K2_GetActorLocation`)) (1.0 0.0 1.0)))))) (+ (.pitch (`KismetMathLibrary.Conv_VectorToRotator` (`KismetMathLibrary.GreaterGreater_VectorRotator` (`KismetMathLibrary.Normal` (* (- (`SceneComponent.K2_GetComponentLocation` (`self.ControllerHand`)) (`self.K2_GetActorLocation`)) (1.0 0.0 1.0)))))) -90.0) (.yaw (`KismetMathLibrary.Conv_VectorToRotator` (`KismetMathLibrary.GreaterGreater_VectorRotator` (`KismetMathLibrary.Normal` (* (- (`SceneComponent.K2_GetComponentLocation` (`self.ControllerHand`)) (`self.K2_GetActorLocation`)) (1.0 0.0 1.0)))))))))
      (:`then_1`
        (if (>= _returnvalue_yaw 0.0)
          (set `self.AmountToMove` -1.0)
          (else
            (set `self.AmountToMove` 1.0)))
        (`self.K2_SetActorLocation` _floor (`KismetMathLibrary.MakeVector` _returnvalue_x_2 _returnvalue_y_2 (+ _returnvalue_z_2 (`self.AmountToMove`))) false false)
        (`self.K2_SetActorLocation` _navmesh (`KismetMathLibrary.MakeVector` _returnvalue_x _returnvalue_y (+ _returnvalue_z (`self.AmountToMove`))) false false)
        (`KismetSystemLibrary.PrintString` (`KismetStringLibrary.Conv_DoubleToString` _returnvalue_z_3))))))

(fn `UserConstructionScript`)